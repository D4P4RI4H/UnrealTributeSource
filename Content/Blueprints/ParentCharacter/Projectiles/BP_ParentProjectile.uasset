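; Parent beam projectile that damages characters and clashes or merges with other beams.
; BeginPlay derives HP and power from the player character's primary attribute, and a looping timer drains HP until the beam expires.
; Sphere overlaps record targets, while Tick uses front and back overlaps to choose clash (stop and damage the other beam) or boost (combine velocity and power, destroying it).
; Boost lacks an ally check; status-effect functions are empty stubs.
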(event `self.Sphere.OnComponentBeginOverlap`
  (params (OverlappedComponent :type "PrimitiveComponent Object Reference") (OtherActor :type "Actor Object Reference") (OtherComp :type "PrimitiveComponent Object Reference") (OtherBodyIndex :type Integer) (bFromSweep :type Boolean) (SweepResult :type "HitResult Structure (by ref)"))
  ;[1 1 1] Collision Events
  (if (and (or (== (`GameplayStatics.GetObjectClass` OtherActor) "/Game/Blueprints/NPC/NPC.NPC_C") (== (`GameplayStatics.GetObjectClass` OtherActor) "BP_ParentProjectile_C")) (!= self OtherActor))
    (set `self.HasOverlapped?` true)
    (bind _asbp_parent_projectile (cast `/Game/Blueprints/ParentCharacter/Projectiles/BP_ParentProjectile` OtherActor)
      (:`then`
        (if (== _asbp_parent_projectile OtherActor)
          (set `self.Overlapped Beam` _asbp_parent_projectile)
          (else
            (bind _asnpc (cast `/Game/Blueprints/NPC/NPC` OtherActor :!label _label)
              (:`then`
                _)
              (:`CastFailed`
                (bind _asbase_character (cast `/Game/Blueprints/ParentCharacter/BaseCharacter` OtherActor))))
            (if (or (== _asnpc OtherActor) (== OtherActor _asbase_character))
              (bind _output_get (set `self.Overlapped Character` OtherActor))
              (`KismetArrayLibrary.Array_AddUnique` (`self.All Overlapped Actors`) _output_get)))))
      (:`CastFailed`
        (goto _label)))))

(event `self.ReceiveBeginPlay`
  ;[1 1 1] Begin Play Event
  (`|ExecutionSequence`
    (:`then_0`
      (bind _asbase_character (cast `/Game/Blueprints/ParentCharacter/BaseCharacter` (`GameplayStatics.GetPlayerCharacter` 0)))
      (set `self.Character` _asbase_character)
      (set `self.Total Intellect` (`/Game/Blueprints/ParentCharacter/BaseCharacter.TotalIntellect` _asbase_character))
      (set `self.Total Strength` (`/Game/Blueprints/ParentCharacter/BaseCharacter.TotalStrength` _asbase_character))
      (set `self.Total Agility` (`/Game/Blueprints/ParentCharacter/BaseCharacter.TotalAgility` _asbase_character)))
    (:`then_1`
      (`self.ProjectilePrimaryAttribute`)
      (bind _output_get (set `self.MaxHP` (* (`self.PrimaryAttribute`) (`self.MaxHP`))))
      (set `self.ProjectilePower` (/ _output_get 10.0))
      (set `self.CurrentHP` (`self.MaxHP`)))
    (:`then_2`
      (`KismetSystemLibrary.K2_SetTimerDelegate` (delegate `LowerBeamHealthOverTime`) 0.1 true)
      (set `self.InitialVelocity` (`MovementComponent.Velocity` (`self.ProjectileMovement`))))
    (:`then_3`
      (`SceneComponent.SetWorldScale3D` (`self.DefaultSceneRoot`) (1.0 1.0 1.0)))))

(event `CustomEvent_3`
  ;[1 1 1] Backup
  (`self.UpdateHealth` 0.01)
  (if (<= (`self.CurrentHP`) 0.01)
    (`self.K2_DestroyActor`)))

(event `self.Sphere.OnComponentEndOverlap`
  (params (OverlappedComponent :type "PrimitiveComponent Object Reference") (OtherActor :type "Actor Object Reference") (OtherComp :type "PrimitiveComponent Object Reference") (OtherBodyIndex :type Integer))
  ;[1 1 1] Collision Events
  (if (and (or (== (`GameplayStatics.GetObjectClass` OtherActor) "/Game/Blueprints/ParentCharacter/Projectiles/BP_ParentProjectile_ChildNew.BP_ParentProjectile_ChildNew_C") (== (`GameplayStatics.GetObjectClass` OtherActor) "BP_ParentProjectile_C")) (!= OtherActor self))
    (`KismetArrayLibrary.Array_RemoveItem` (`self.All Overlapped Actors`) OtherActor)
    (if (not (or (`KismetSystemLibrary.IsValid` (`self.Overlapped Beam`)) (`KismetSystemLibrary.IsValid` (`self.Overlapped Character`))))
      (set `self.HasOverlapped?` false)
      (set `self.Overlapped Character` null)
      (set `self.Overlapped Beam` null))))

(event `LowerBeamHealthOverTime`
  ;[1 1 1] Begin Play Event
  (`self.UpdateHealth` 0.05)
  (if (<= (`self.CurrentHP`) 0.01)
    (`self.K2_DestroyActor`)))

(event `self.BeamFront.OnComponentBeginOverlap`
  (params (OverlappedComponent :type "PrimitiveComponent Object Reference") (OtherActor :type "Actor Object Reference") (OtherComp :type "PrimitiveComponent Object Reference") (OtherBodyIndex :type Integer) (bFromSweep :type Boolean) (SweepResult :type "HitResult Structure (by ref)"))
  ;[1 1 1] Collision Events
  (if (and (or (== (`GameplayStatics.GetObjectClass` OtherActor) "/Game/Blueprints/NPC/NPC.NPC_C") (== (`GameplayStatics.GetObjectClass` OtherActor) "BP_ParentProjectile_C")) (!= self OtherActor))
    (set `self.OverlappedFront` true)))

(event `self.BeamFront.OnComponentEndOverlap`
  (params (OverlappedComponent :type "PrimitiveComponent Object Reference") (OtherActor :type "Actor Object Reference") (OtherComp :type "PrimitiveComponent Object Reference") (OtherBodyIndex :type Integer))
  ;[1 1 1] Collision Events
  (if (and (or (== (`GameplayStatics.GetObjectClass` OtherActor) "/Game/Blueprints/NPC/NPC.NPC_C") (== (`GameplayStatics.GetObjectClass` OtherActor) "BP_ParentProjectile_C")) (!= self OtherActor))
    (set `self.OverlappedFront` false)))

(event `ProjectileAction`
  ;[1 1 1] Tick Event
  (if (or (== (`GameplayStatics.GetObjectClass` (`self.Overlapped Beam`)) "BP_ParentProjectile_C") (== (`GameplayStatics.GetObjectClass` (`self.Overlapped Character`)) "/Game/Blueprints/ParentCharacter/BaseCharacter.BaseCharacter_C") (== (`GameplayStatics.GetObjectClass` (`self.Overlapped Character`)) "/Game/Blueprints/NPC/NPC.NPC_C")) :!label _label_2
    ;;[1 1 1] Decide to clash or boost
    (if (`self.HasOverlapped?`)
      (if (`self.OverlappedFront`)
        (`|ExecutionSequence`
          (:`then_0`
            (`self.ProjectileClash`))
          (:`then_1`
            (`self.DamageCharacter`)))
        (elif (`self.OverlappedBack`)
          (`|ExecutionSequence`
            (:`then_0`
              (`self.ProjectileBoost`))
            (:`then_1`
              (`self.DamageCharacter`)))
          (else
            (set `self.Overlapped Beam` null)
            (set `self.Overlapped Character` null)
            (`KismetArrayLibrary.Array_Clear` (`self.All Overlapped Actors`))))))
    (else
      ;;[1 1 1] Return to normal speed
      (set `MovementComponent.Velocity` (`self.InitialVelocity`) (`self.ProjectileMovement`))
      (`SceneComponent.SetVisibility` (`self.P_Trail`) true false))))

(event `self.ReceiveTick`
  (params (DeltaSeconds :type "Float (single-precision)"))
  ;[1 1 1] Tick Event
  (goto _label_2))

(event `self.BeamBack.OnComponentBeginOverlap`
  (params (OverlappedComponent :type "PrimitiveComponent Object Reference") (OtherActor :type "Actor Object Reference") (OtherComp :type "PrimitiveComponent Object Reference") (OtherBodyIndex :type Integer) (bFromSweep :type Boolean) (SweepResult :type "HitResult Structure (by ref)"))
  ;[1 1 1] Collision Events
  (if (and (or (== (`GameplayStatics.GetObjectClass` OtherActor) "/Game/Blueprints/NPC/NPC.NPC_C") (== (`GameplayStatics.GetObjectClass` OtherActor) "BP_ParentProjectile_C")) (!= self OtherActor))
    (set `self.OverlappedBack` true)))

(event `self.BeamBack.OnComponentEndOverlap`
  (params (OverlappedComponent :type "PrimitiveComponent Object Reference") (OtherActor :type "Actor Object Reference") (OtherComp :type "PrimitiveComponent Object Reference") (OtherBodyIndex :type Integer))
  ;[1 1 1] Collision Events
  (if (and (or (== (`GameplayStatics.GetObjectClass` OtherActor) "/Game/Blueprints/NPC/NPC.NPC_C") (== (`GameplayStatics.GetObjectClass` OtherActor) "BP_ParentProjectile_C")) (!= self OtherActor))
    (set `self.OverlappedBack` false)))

(fn `ApplyBurn`)

(fn `ApplyParalyze`)

(fn `ApplyPoison`)

(fn `ApplySlow`)

(fn `ApplyStun`)

(fn `DamageCharacter`
  (for _array_element (`self.All Overlapped Actors`)
    (if (== _array_element (`self.Overlapped Character`))
      (`GameplayStatics.ApplyDamage` (`self.Overlapped Character`) (`self.ProjectilePower`) null (`self.GetOwner`)))))

(fn `ProjectileBoost`
  (bind _overlapped_beam (`self.Overlapped Beam`))
  ;[1 1 1] Need to place check to see if beam is allied
  (set `self.Being Powered Up` true)
  (bind _asbp_parent_projectile (cast `/Game/Blueprints/ParentCharacter/Projectiles/BP_ParentProjectile` _overlapped_beam))
  (if (== _asbp_parent_projectile _overlapped_beam)
    (`self.UpdateHealth` _asbp_parent_projectile (* -1 (`/Game/Blueprints/ParentCharacter/Projectiles/BP_ParentProjectile.CurrentHP` _asbp_parent_projectile)))
    (bind _output_get (set `MovementComponent.Velocity` (+ (`/Game/Blueprints/ParentCharacter/Projectiles/BP_ParentProjectile.InitialVelocity` _asbp_parent_projectile) (`self.InitialVelocity`)) (`/Game/Blueprints/ParentCharacter/Projectiles/BP_ParentProjectile.ProjectileMovement` _asbp_parent_projectile)))
    (bind _output_get_2 (set `MovementComponent.Velocity` _output_get (`self.ProjectileMovement`)))
    (set `self.ProjectilePower` (+ (`self.ProjectilePower`) (`/Game/Blueprints/ParentCharacter/Projectiles/BP_ParentProjectile.ProjectilePower` _asbp_parent_projectile)))
    (`SceneComponent.SetVisibility` (`self.P_Trail`) true false)
    (`self.K2_DestroyActor` _asbp_parent_projectile)))

(fn `ProjectileClash`
  (bind _overlapped_beam (`self.Overlapped Beam`))
  (bind _asbp_parent_projectile (cast `/Game/Blueprints/ParentCharacter/Projectiles/BP_ParentProjectile` _overlapped_beam))
  (if (== (`GameplayStatics.GetObjectClass` _asbp_parent_projectile) (`GameplayStatics.GetObjectClass` _overlapped_beam))
    (if (and (`/Game/Blueprints/ParentCharacter/Projectiles/BP_ParentProjectile.OverlappedFront` _asbp_parent_projectile) (`self.OverlappedFront`))
      _
      (else
        _))
    (set `MovementComponent.Velocity` (0.0 0.0 0.0) (`/Game/Blueprints/ParentCharacter/Projectiles/BP_ParentProjectile.ProjectileMovement` _asbp_parent_projectile))
    (set `MovementComponent.Velocity` (0.0 0.0 0.0) (`self.ProjectileMovement`))
    (`SceneComponent.SetVisibility` (`self.P_Trail`) false false)
    (bind _returnvalue (`GameplayStatics.ApplyDamage` (`self.Overlapped Beam`) (`self.ProjectilePower`) null (`self.GetOwner`)))
    (`self.UpdateHealth` _returnvalue)
    (if (<= (`/Game/Blueprints/ParentCharacter/Projectiles/BP_ParentProjectile.CurrentHP` _asbp_parent_projectile) 0.0)
      (`self.K2_DestroyActor` (`self.Overlapped Beam`))
      (set `MovementComponent.Velocity` (`self.InitialVelocity`) (`self.ProjectileMovement`))
      (`SceneComponent.SetVisibility` (`self.P_Trail`) true false))))

(fn `ProjectilePrimaryAttribute`
  (bind _primaryattribute (`/Game/Blueprints/ParentCharacter/BaseCharacter.PrimaryAttribute` (`self.Character`)))
  (if (`KismetStringLibrary.EqualEqual_StrStr` _primaryattribute "Strength")
    (set `self.PrimaryAttribute` (`self.Total Strength`))
    (elif (`KismetStringLibrary.EqualEqual_StrStr` _primaryattribute "Agility")
      (set `self.PrimaryAttribute` (`self.Total Agility`))
      (elif (`KismetStringLibrary.EqualEqual_StrStr` _primaryattribute "Intellect")
        (set `self.PrimaryAttribute` (`self.Total Intellect`))))))

(fn `UpdateHealth`
  (params (DeltaDamage :type "Float (double-precision)"))
  (set `self.CurrentHP` (`KismetMathLibrary.FClamp` (- (`self.CurrentHP`) DeltaDamage) 0.0 (`self.MaxHP`))))

(fn `UserConstructionScript`)