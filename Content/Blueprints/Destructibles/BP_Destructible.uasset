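; Destructible prop that breaks in stages when hit by a projectile or damaged, then respawns after a countdown.
; Health counts hits upward: the first two hide break meshes, and the third fires ItemDrop and SetRespawn.
; ItemDrop only calls RemoveFromWorld, which hides remaining meshes and disables collision without destroying the actor.
; A looping one-second timer decrements Timer, then restores visibility, collision and Health at zero.
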(event `self.ReceiveBeginPlay`)

(event `self.Box.OnComponentBeginOverlap`
  (params (OverlappedComponent :type "PrimitiveComponent Object Reference") (OtherActor :type "Actor Object Reference") (OtherComp :type "PrimitiveComponent Object Reference") (OtherBodyIndex :type Integer) (bFromSweep :type Boolean) (SweepResult :type "HitResult Structure (by ref)"))
  (bind _returnvalue (== (`GameplayStatics.GetObjectClass` OtherActor) "/Game/Blueprints/ParentCharacter/Projectiles/BP_ParentProjectile.BP_ParentProjectile_C"))
  (if _returnvalue
    (if _returnvalue
      (if (> 3 (`self.Health`))
        (`self.K2_DestroyActor` OtherActor)
        (switch `int` (`self.Health`) :!label _label
          (:`0`
            (`SceneComponent.SetVisibility` (`self.BreakOne`) false false)
            (set `self.Health` 1))
          (:`1`
            (`SceneComponent.SetVisibility` (`self.BreakTwo`) false false)
            (set `self.Health` 2))
          (:`2`
            (set `self.Health` 3)
            (`self.ItemDrop`)
            (`self.SetRespawn`))))
      (else
        (goto _label)))))

(event `self.ReceiveAnyDamage`
  (params (Damage :type "Float (single-precision)") (DamageType :type "DamageType Object Reference") (InstigatedBy :type "Controller Object Reference") (DamageCauser :type "Actor Object Reference"))
  (goto _label))

(event `ItemDrop`
  (`self.RemoveFromWorld`))

(event `SetRespawn`
  (`KismetSystemLibrary.K2_SetTimerDelegate` (delegate `RespawnTimer`) 1.0 true))

(event `RespawnTimer`
  (bind _main (`self.Main`))
  (`/Engine/EditorBlueprintResources/StandardMacros.DecrementInt` (`self.Timer`)
    (:`  `
      (if (<= (`self.Timer`) 0)
        (`KismetSystemLibrary.K2_ClearTimer` null "RespawnTimer")
        (set `self.Timer` 10)
        (set `self.Health` 0)
        (`SceneComponent.SetVisibility` (`self.BreakOne`) true false)
        (`SceneComponent.SetVisibility` (`self.BreakTwo`) true false)
        (`PrimitiveComponent.SetCollisionEnabled` _main "QueryAndPhysics")
        (`SceneComponent.SetVisibility` _main true false)
        (`SceneComponent.SetVisibility` (`self.AestheticOne`) true false)
        (`SceneComponent.SetVisibility` (`self.AestheticTwo`) true false)
        (`SceneComponent.SetVisibility` (`self.AestheticThree`) true false)
        (`PrimitiveComponent.SetCollisionEnabled` (`self.SkeletalMesh`) "QueryAndPhysics")))))

(fn `RemoveFromWorld`
  (bind _main (`self.Main`))
  (`PrimitiveComponent.SetCollisionEnabled` _main "NoCollision")
  (`SceneComponent.SetVisibility` _main false false)
  (`SceneComponent.SetVisibility` (`self.AestheticOne`) false false)
  (`SceneComponent.SetVisibility` (`self.AestheticTwo`) false false)
  (`SceneComponent.SetVisibility` (`self.AestheticThree`) false false)
  (`PrimitiveComponent.SetCollisionEnabled` (`self.SkeletalMesh`) "NoCollision"))

(fn `UserConstructionScript`)