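; BP_Destructible_Child is an explosive destructible that damages actors around it when its ItemDrop event fires.
; ItemDrop flashes the DestructibleColor parameter on its four mesh components between red and grey twice, then calls RemoveFromWorld.
; It then asks GS_UnrealTribute to spawn a line-of-sight area effect at its location, with debug drawing, passing DamageTargets as the hit delegate to apply damage.
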(event `self.ItemDrop`
  (`MeshComponent.SetVectorParameterValueOnMaterials` (`self.Main`) "DestructibleColor" (1.0 0.0 0.0))
  (`MeshComponent.SetVectorParameterValueOnMaterials` (`self.AestheticOne`) "DestructibleColor" (1.0 0.0 0.0))
  (`MeshComponent.SetVectorParameterValueOnMaterials` (`self.AestheticTwo`) "DestructibleColor" (1.0 0.0 0.0))
  (`MeshComponent.SetVectorParameterValueOnMaterials` (`self.AestheticThree`) "DestructibleColor" (1.0 0.0 0.0))
  (`KismetSystemLibrary.Delay` 0.5)
  (`MeshComponent.SetVectorParameterValueOnMaterials` (`self.Main`) "DestructibleColor" (0.18 0.18 0.18))
  (`MeshComponent.SetVectorParameterValueOnMaterials` (`self.AestheticOne`) "DestructibleColor" (0.18 0.18 0.18))
  (`MeshComponent.SetVectorParameterValueOnMaterials` (`self.AestheticTwo`) "DestructibleColor" (0.18 0.18 0.18))
  (`MeshComponent.SetVectorParameterValueOnMaterials` (`self.AestheticThree`) "DestructibleColor" (0.18 0.18 0.18))
  (`KismetSystemLibrary.Delay` 0.5)
  (`MeshComponent.SetVectorParameterValueOnMaterials` (`self.Main`) "DestructibleColor" (1.0 0.0 0.0))
  (`MeshComponent.SetVectorParameterValueOnMaterials` (`self.AestheticOne`) "DestructibleColor" (1.0 0.0 0.0))
  (`MeshComponent.SetVectorParameterValueOnMaterials` (`self.AestheticTwo`) "DestructibleColor" (1.0 0.0 0.0))
  (`MeshComponent.SetVectorParameterValueOnMaterials` (`self.AestheticThree`) "DestructibleColor" (1.0 0.0 0.0))
  (`KismetSystemLibrary.Delay` 0.5)
  (`MeshComponent.SetVectorParameterValueOnMaterials` (`self.Main`) "DestructibleColor" (0.18 0.18 0.18))
  (`MeshComponent.SetVectorParameterValueOnMaterials` (`self.AestheticOne`) "DestructibleColor" (0.18 0.18 0.18))
  (`MeshComponent.SetVectorParameterValueOnMaterials` (`self.AestheticTwo`) "DestructibleColor" (0.18 0.18 0.18))
  (`MeshComponent.SetVectorParameterValueOnMaterials` (`self.AestheticThree`) "DestructibleColor" (0.18 0.18 0.18))
  (`KismetSystemLibrary.Delay` 0.5)
  (`self.RemoveFromWorld`)
  (bind _asgs_unreal_tribute (cast `/Game/Blueprints/GS_UnrealTribute` (`GameplayStatics.GetGameState`)))
  (`/Game/Blueprints/GS_UnrealTribute.SpawnAOE` _asgs_unreal_tribute (`self.K2_GetActorLocation`) 400.0 true null (delegate `DamageTargets`) 5.0 (struct :`R` 1.0 :`G` 0.87942 :`A` 1.0)))

(event `DamageTargets`
  (params (`Hit Actor` :type "Actor Object Reference"))
  (`GameplayStatics.ApplyDamage` `Hit Actor` 0.7 null self))

(fn `UserConstructionScript`
  (`parent.UserConstructionScript`))