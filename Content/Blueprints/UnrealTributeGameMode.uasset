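; Game mode for an Unreal tribute game that sets up joining players and handles player and creep respawns.
; On login it has the player controller draw its HUD client-side and, with authority, records the controller in a list.
; Respawn hands a spawn transform to the controller's server respawn, while RespawnCreeps spawns an NPC with its behavior tree and initializes its AI.
; Delay and possess nodes are left disconnected, so creeps spawn immediately.
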(event `self.K2_PostLogin`
  (params (NewPlayer :type "PlayerController Object Reference"))
  (bind _asunreal_tribute_controller (cast `/Game/Blueprints/ParentCharacter/UnrealTributeController` NewPlayer))
  (`/Game/Blueprints/ParentCharacter/UnrealTributeController.Client_DrawHUD` _asunreal_tribute_controller))

(event `Respawn`
  (params (Controller :type "/Game/Blueprints/ParentCharacter/UnrealTributeController Object Reference"))
  (`/Game/Blueprints/ParentCharacter/UnrealTributeController.Server_Respawn` Controller (`self.Spawn Transform`)))

(event `Respawn Creeps`
  (params (SpawnLoc :type "Vector Structure") (AIController :type "Controller Object Reference"))
  (bind _returnvalue (`AIBlueprintHelperLibrary.SpawnAIFromClass` "/Game/Blueprints/NPC/NPC.NPC_C" "/Game/Blueprints/NPC/BT_NPC.BT_NPC" SpawnLoc (struct) true null))
  (bind _asnpc (cast `/Game/Blueprints/NPC/NPC` _returnvalue))
  (`/Game/Blueprints/NPC/NPC.SetUpAI` _asnpc))

(event `Event OnPostLogin`
  (params (NewItem :type "/Game/Blueprints/ParentCharacter/UnrealTributeController Object Reference (by ref)"))
  (`/Engine/EditorBlueprintResources/ActorMacros.Switch Has Authority`
    (:`Authority`
      (`KismetArrayLibrary.Array_Add` (`self.AllPlayerController`) NewItem))))

(fn `UserConstructionScript`)