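; AI controller for NPCs that runs the BT_NPC behavior tree on BeginPlay or through a RunBT event.
; AI perception updates set the CanSeePlayer blackboard key to true for any BaseCharacter, without checking the stimulus or ever clearing the key.
; CombatantDied is a respawn routine that spawns an AI pawn from the given type at a supplied location with BT_NPC, then has the passed controller possess it.
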(event `Run BT`
  (`self.RunBehaviorTree` "/Game/Blueprints/NPC/BT_NPC.BT_NPC"))

(event `self.ReceiveBeginPlay`
  (`self.RunBehaviorTree` "/Game/Blueprints/NPC/BT_NPC.BT_NPC"))

(event `self.AIPerception.OnTargetPerceptionUpdated`
  (params (Actor :type "Actor Object Reference") (Stimulus :type "AIStimulus Structure"))
  (bind _ascharacter (cast `Character` Actor))
  (cast `/Game/Blueprints/ParentCharacter/BaseCharacter` _ascharacter)
  (`BlackboardComponent.SetValueAsBool` (`AIBlueprintHelperLibrary.GetBlackboard` null) "CanSeePlayer" true))

(fn `CombatantDied`
  (params (Type :type "Object Object Reference") (Controller :type "Controller Object Reference") (SpawnLoc :type "Vector Structure"))
  (bind _aspawn (castclass `Pawn` (`GameplayStatics.GetObjectClass` Type)))
  (bind _returnvalue (`AIBlueprintHelperLibrary.SpawnAIFromClass` _aspawn "/Game/Blueprints/NPC/BT_NPC.BT_NPC" SpawnLoc (struct) false null))
  (`self.Possess` Controller _returnvalue))

(fn `UserConstructionScript`)