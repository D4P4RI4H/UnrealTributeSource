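; AI-controlled NPC creep that fights with melee, rewards its killer and respawns through the game mode.
; Health scales with Strength at BeginPlay, and damage updates a health bar widget.
; Melee plays a montage and immediately sphere-traces at its Sphere component to apply damage.
; Death unpossesses, ragdolls, grants killer stats and XP with power-curve leveling, then requests a respawn at the spawn location; FightDirector hooks are disconnected.
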(event `self.ReceiveAnyDamage`
  (params (Damage :type "Float (single-precision)") (DamageType :type "DamageType Object Reference") (InstigatedBy :type "Controller Object Reference") (DamageCauser :type "Actor Object Reference"))
  (bind _currenthp (`self.CurrentHp`))
  (if (not (`self.IsDead?`))
    (`self.UpdateHealth` Damage)
    (bind _asw_dummy_hp (cast `/Game/Blueprints/NPC/Widgets/W_DummyHP` (`WidgetComponent.GetUserWidgetObject` (`self.HealthBar`))))
    (set `/Game/Blueprints/NPC/Widgets/W_DummyHP.CurrentHp` _currenthp _asw_dummy_hp)
    (set `/Game/Blueprints/NPC/Widgets/W_DummyHP.MaxHp` (`self.MaxHp`) _asw_dummy_hp)
    (if (< _currenthp 0.01)
      (`self.Death` DamageCauser))))

(event `self.ReceiveBeginPlay`
  (`self.SetUpAI`)
  (`self.ScaleHealth`)
  (bind _asai_npc (cast `/Game/Blueprints/NPC/AI_NPC` (`self.GetController`)))
  (set `self.As AI NPC` _asai_npc))

(event `/Game/Blueprints/NPC/I_NPCFunctions.MeleeAttack`
  (bind _returnvalue (`SceneComponent.K2_GetComponentLocation` (`self.Sphere`)))
  (`|PlayMontage` (`self.Mesh`) "/Game/Blueprints/NPC/Attack_PrimaryA_Montage.Attack_PrimaryA_Montage"
    (:`then`
      (bind _outhit (`KismetSystemLibrary.SphereTraceSingle` _returnvalue _returnvalue 50.0 "TraceTypeQuery1" false (`self.GetAllChildActors` true) "ForDuration"))
      (bind (_bblockinghit _binitialoverlap _time _distance _location _impactpoint _normal _impactnormal _physmat _hitactor) (`GameplayStatics.BreakHitResult` _outhit))
      (bind _ascharacter (cast `Character` _hitactor))
      (`/Engine/EditorBlueprintResources/StandardMacros.IsValid` _ascharacter
        (:`Is Valid`
          (if (not (== _ascharacter "NPC"))
            (`GameplayStatics.ApplyDamage` _hitactor 0.1 null self)))))))

(event `Death`
  (params (Object :type "Object Object Reference"))
  (bind _mesh (`self.Mesh`))
  (`Controller.UnPossess` (`AIBlueprintHelperLibrary.GetAIController` self))
  (`PrimitiveComponent.SetCollisionEnabled` _mesh "PhysicsOnly")
  (`PrimitiveComponent.SetSimulatePhysics` _mesh true)
  (`PrimitiveComponent.SetCollisionEnabled` (`self.CapsuleComponent`) "NoCollision")
  (`self.SetLifeSpan` 3.0)
  (`SceneComponent.SetVisibility` (`self.HealthBar`) false false)
  (`self.UpdateKillerStats` Object)
  (`self.UpdateKillerXp` Object)
  (set `self.IsDead?` true)
  (bind _asunreal_tribute_game_mode (cast `/Game/Blueprints/UnrealTributeGameMode` (`GameplayStatics.GetGameMode`)))
  (`/Game/Blueprints/UnrealTributeGameMode.Respawn Creeps` _asunreal_tribute_game_mode (`self.Spawn Location`) (`self.GetController`)))

(event `Set Health Regen`
  (`self.UpdateHealth` 0.0))

(event `SetUpAI`
  (set `self.CurrentHp` (`self.MaxHp`))
  (set `self.Spawn Location` (`self.K2_GetActorLocation`)))

(fn `ScaleHealth`
  (set `self.CurrentHp` (* (`self.Strength`) (`self.CurrentHp`)))
  (set `self.MaxHp` (* (`self.Strength`) (`self.MaxHp`))))

(fn `UpdateHealth`
  (params (DeltaHp :type "Float (double-precision)"))
  (bind _output_get (set `self.CurrentHp` (`KismetMathLibrary.FClamp` (- (`self.CurrentHp`) DeltaHp) 0.0 (`self.MaxHp`))))
  (`KismetSystemLibrary.PrintString` (`KismetStringLibrary.Conv_DoubleToString` _output_get)))

(fn `UpdateKillerStats`
  (params (Object :type "Object Object Reference"))
  (bind _asbase_character (cast `/Game/Blueprints/ParentCharacter/BaseCharacter` Object)
    (:`then`
      (bind _output_get (set `/Game/Blueprints/ParentCharacter/BaseCharacter.Intelligence` (+ (`/Game/Blueprints/ParentCharacter/BaseCharacter.Intelligence` _asbase_character) (`self.StatWorth`)) _asbase_character))
      (bind _output_get_2 (set `/Game/Blueprints/ParentCharacter/BaseCharacter.Agility` (+ (`/Game/Blueprints/ParentCharacter/BaseCharacter.Agility` _asbase_character) (`self.StatWorth`)) _asbase_character))
      (bind _output_get_3 (set `/Game/Blueprints/ParentCharacter/BaseCharacter.Strength` (+ (`/Game/Blueprints/ParentCharacter/BaseCharacter.Strength` _asbase_character) (`self.StatWorth`)) _asbase_character)))
    (:`CastFailed`
      (cast `/Game/Blueprints/ParentCharacter/UnrealTributeController` Object)
      (`KismetSystemLibrary.PrintString` "Controller"))))

(fn `UpdateKillerXp`
  (params (Object :type "Object Object Reference"))
  (locals (CarryOverXp :type "Float (double-precision)"))
  (bind _asbase_character (cast `/Game/Blueprints/ParentCharacter/BaseCharacter` Object))
  (bind _currentxp (`/Game/Blueprints/ParentCharacter/BaseCharacter.CurrentXp` _asbase_character))
  (bind _output_get (set `/Game/Blueprints/ParentCharacter/BaseCharacter.CurrentXp` (+ _currentxp (* (`/Game/Blueprints/ParentCharacter/BaseCharacter.PlayerLevel` _asbase_character) (`self.ExperienceWorth`))) _asbase_character))
  (bind _maxxp (`/Game/Blueprints/ParentCharacter/BaseCharacter.MaxXp` _asbase_character))
  (if (>= _output_get _maxxp)
    (bind _output_get_2 (set `local.CarryOverXp` (- _currentxp _maxxp)))
    (bind _playerlevel (`/Game/Blueprints/ParentCharacter/BaseCharacter.PlayerLevel` _asbase_character))
    ;[1 1 1] Level Up
    (bind _result (`/Engine/EditorBlueprintResources/StandardMacros.IncrementInt` _playerlevel)
      (:`  `
        (set `/Game/Blueprints/ParentCharacter/BaseCharacter.PlayerLevel` _result _asbase_character)
        (set `/Game/Blueprints/ParentCharacter/BaseCharacter.MaxXp` (`KismetMathLibrary.Conv_IntToDouble` (+ (`KismetMathLibrary.FTrunc` _maxxp) (`KismetMathLibrary.FTrunc` (`KismetMathLibrary.MultiplyMultiply_FloatFloat` (`KismetMathLibrary.Conv_IntToDouble` _playerlevel) 2.4)))) _asbase_character)
        (set `/Game/Blueprints/ParentCharacter/BaseCharacter.CurrentXp` _output_get_2 _asbase_character)
        (`KismetSystemLibrary.PrintString` (`KismetStringLibrary.Conv_IntToString` _playerlevel))))
    (else
      (`KismetSystemLibrary.PrintString` "Hello"))))

(fn `UserConstructionScript`
  (`SceneComponent.SetVisibility` (`self.Sphere`) false false))