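; BP_DummyTarget is a damageable dummy that grants Intelligence, Agility and Strength to its BaseCharacter killer, then destroys itself.
; BeginPlay scales health by Strength and starts a looping "regen" timer that only re-clamps HP.
; AnyDamage sets IsDead on the first hit, blocking later hits.
; It loops over all dummies, damaging itself once per dummy, syncing each health widget and checking its own HP for death.
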(event `self.ReceiveBeginPlay`
  (`self.ScaleHealth`)
  (`KismetSystemLibrary.K2_SetTimerDelegate` (delegate `Set Health Regen`) 0.1 true)
  (bind _returnvalue (`GameplayStatics.GetActorOfClass` "/Game/Blueprints/ParentAI/FightDirector.FightDirector_C"))
  (set `self.FightDirector` _returnvalue))

(event `Set Health Regen`
  (`self.UpdateHealth` 0.0))

(event `self.ReceiveAnyDamage`
  (params (Damage :type "Float (single-precision)") (DamageType :type "DamageType Object Reference") (InstigatedBy :type "Controller Object Reference") (DamageCauser :type "Actor Object Reference"))
  (if (not (`self.IsDead?`))
    (set `self.IsDead?` true)
    (bind _outactors (`GameplayStatics.GetAllActorsOfClass` "BP_DummyTarget_C"))
    (for _array_element _outactors
      (`self.UpdateHealth` Damage)
      (bind _asw_dummy_hp (cast `/Game/Blueprints/NPC/Widgets/W_DummyHP` (`WidgetComponent.GetUserWidgetObject` (`/Game/Blueprints/ParentAI/BP_DummyTarget.Widget` _array_element))))
      (set `/Game/Blueprints/NPC/Widgets/W_DummyHP.CurrentHp` (`/Game/Blueprints/ParentAI/BP_DummyTarget.CurrentHp` _array_element) _asw_dummy_hp)
      (set `/Game/Blueprints/NPC/Widgets/W_DummyHP.MaxHp` (`/Game/Blueprints/ParentAI/BP_DummyTarget.MaxHp` _array_element) _asw_dummy_hp)
      (if (<= (`self.CurrentHp`) 0.01)
        (`KismetSystemLibrary.PrintString` (`KismetSystemLibrary.GetDisplayName` _array_element))
        (`self.UpdateKillerStats` DamageCauser)
        (`PrimitiveComponent.SetCollisionEnabled` (`self.SkeletalMesh`) "NoCollision")
        (`PrimitiveComponent.SetCollisionEnabled` (`self.Capsule`) "NoCollision")
        (`self.K2_DestroyActor`)))))

(fn `ScaleHealth`
  (set `self.CurrentHp` (* (`self.Strength`) (`self.CurrentHp`)))
  (set `self.MaxHp` (* (`self.Strength`) (`self.MaxHp`))))

(fn `UpdateHealth`
  (params (DeltaHp :type "Float (double-precision)"))
  (set `self.CurrentHp` (`KismetMathLibrary.FClamp` (- (`self.CurrentHp`) DeltaHp) 0.0 (`self.MaxHp`))))

(fn `UpdateKillerStats`
  (params (Object :type "Object Object Reference"))
  (bind _asbase_character (cast `/Game/Blueprints/ParentCharacter/BaseCharacter` Object))
  (set `/Game/Blueprints/ParentCharacter/BaseCharacter.Intelligence` (+ (`/Game/Blueprints/ParentCharacter/BaseCharacter.Intelligence` _asbase_character) (`self.StatWorth`)) _asbase_character)
  (set `/Game/Blueprints/ParentCharacter/BaseCharacter.Agility` (+ (`/Game/Blueprints/ParentCharacter/BaseCharacter.Agility` _asbase_character) (`self.StatWorth`)) _asbase_character)
  (set `/Game/Blueprints/ParentCharacter/BaseCharacter.Strength` (+ (`/Game/Blueprints/ParentCharacter/BaseCharacter.Strength` _asbase_character) (`self.StatWorth`)) _asbase_character))

(fn `UserConstructionScript`)