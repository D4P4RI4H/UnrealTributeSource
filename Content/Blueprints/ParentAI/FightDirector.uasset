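; Fight director that decides which NPC performs the next melee attack on a looping timer.
; Each tick multiplies enemy grades by a facing factor, favouring those facing opposite the player's forward vector.
; The top-graded enemy's AI_NPC controller gets the attack message, then its grade is re-rolled randomly.
; Dead AI are removed from tracking; initial grade seeding and debug widget creation are disconnected.
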(event `self.ReceiveBeginPlay`
  (set `self.CustomTimeDilation` 1.0)
  (bind _outactors (`GameplayStatics.GetAllActorsOfClass` "/Game/Blueprints/NPC/NPC.NPC_C"))
  (set `self.EnemyList` _outactors)
  (for _ (`self.EnemyList`)
    _)
  (`KismetSystemLibrary.K2_SetTimerDelegate` (delegate `Trigger Attack`) (`self.TimeBetweenAttacks`) true))

(event `AI_died`
  (params (DeadAI :type "/Game/Blueprints/NPC/NPC Object Reference"))
  (`KismetArrayLibrary.Array_RemoveItem` (`self.EnemyList`) DeadAI)
  (`BlueprintMapLibrary.Map_Remove` (`self.EnemyGrading`) DeadAI))

(event `Trigger Attack`
  (`self.RecalculateScores`)
  (bind (_loc_highestvalue1 _loc_highestgradedai1) (`self.FindHighestGrade`))
  (bind _asai_npc (cast `/Game/Blueprints/NPC/AI_NPC` (`AIBlueprintHelperLibrary.GetAIController` _loc_highestgradedai1))
    (:`then`
      (message `/Game/Blueprints/NPC/I_NPCFunctions.MeleeAttack` _asai_npc)
      (`BlueprintMapLibrary.Map_Add` (`self.EnemyGrading`) _loc_highestgradedai1 (`KismetMathLibrary.RandomFloatInRange` 1.0 5.0))
      (`self.UpdateDebugWidgets` _loc_highestgradedai1))
    (:`CastFailed`
      (`KismetSystemLibrary.PrintString` "CastFailed (meleeEnemyFightDirector)" true true (struct :`R` 1.0 :`G` 0.020335 :`B` 0.762118 :`A` 1.0)))))

(fn `AddDebugWidgets`
  (params (EnemyInstance :type "/Game/Blueprints/NPC/NPC Object Reference (by ref)"))
  (locals (Loc_Widget :type "/Game/Blueprints/NPC/Widgets/W_DebugEnemyAI Object Reference"))
  (`BlueprintMapLibrary.Map_Add` (`self.EnemyGrading`) EnemyInstance (`KismetMathLibrary.RandomFloatInRange` 1.0 5.0)))

(fn `FindHighestGrade`
  (returns (Loc_HighestValue1 :type "Float (double-precision)") (Loc_HighestGradedAI1 :type "/Game/Blueprints/NPC/NPC Object Reference"))
  (locals (Loc_HighestValue :type "Float (double-precision)") (Loc_HighestGradedAI :type "/Game/Blueprints/NPC/NPC Object Reference"))
  (bind _keys (`BlueprintMapLibrary.Map_Keys` (`self.EnemyGrading`)))
  (for _array_element _keys
    (bind _value (`BlueprintMapLibrary.Map_Find` (`self.EnemyGrading`) _array_element))
    (if (> _value (`local.Loc_HighestValue`))
      (set `local.Loc_HighestValue` _value)
      (set `local.Loc_HighestGradedAI` _array_element)))
  (return (`local.Loc_HighestValue`) (`local.Loc_HighestGradedAI`)))

(fn `RecalculateScores`
  (`self.ScoreByPosition`))

(fn `ScoreByPosition`
  (bind _enemygrading (`self.EnemyGrading`))
  (for _array_element (`self.EnemyList`)
    (`BlueprintMapLibrary.Map_Add` _enemygrading _array_element (* (`BlueprintMapLibrary.Map_Find` _enemygrading _array_element) (+ (`KismetMathLibrary.NormalizeToRange` (* (`KismetMathLibrary.Dot_VectorVector` (`self.GetActorForwardVector` _array_element) (`self.GetActorForwardVector` (`GameplayStatics.GetPlayerCharacter` 0))) -1.0) -1.0 1.0) 0.5)))))

(fn `UpdateDebugWidgets`
  (params (EnemyInstance :type "/Game/Blueprints/NPC/NPC Object Reference"))
  (set `/Game/Blueprints/NPC/Widgets/W_DebugEnemyAI.FightingGrade` (`BlueprintMapLibrary.Map_Find` (`self.EnemyGrading`) EnemyInstance) (`BlueprintMapLibrary.Map_Find` (`self.EnemyWidgets`) EnemyInstance)))

(fn `UserConstructionScript`)