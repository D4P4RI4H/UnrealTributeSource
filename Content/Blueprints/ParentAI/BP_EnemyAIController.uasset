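; AI controller for enemy NPCs that starts BT_EnemyAI and feeds its blackboard.
; On BeginPlay it caches the controlled NPC, stores player 0 as CurrentTarget and writes the initial AIState.
; AI perception updates set CanSeeTarget from whether the stimulus was sensed, without filtering by actor.
; AIAttack switches the AIState enum, while Pawn_Attack separately triggers the NPC's melee attack.
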(event `self.ReceiveBeginPlay`
  (`self.RunBehaviorTree` "/Game/Blueprints/ParentAI/BT_EnemyAI.BT_EnemyAI")
  (bind _asnpc (cast `/Game/Blueprints/NPC/NPC` (`self.K2_GetPawn`)))
  (set `self.NPC` _asnpc)
  (set `self.CurrentTarget` (`GameplayStatics.GetPlayerCharacter` 0))
  (`BlackboardComponent.SetValueAsEnum` (`AIBlueprintHelperLibrary.GetBlackboard` null) "AIState" (`self.CurrentState`)))

(event `AIAttack`
  (bind _output_get (set `self.CurrentState` "NewEnumerator1"))
  (`BlackboardComponent.SetValueAsEnum` (`AIBlueprintHelperLibrary.GetBlackboard` null) "AIState" _output_get))

(event `Pawn_Attack`
  (`/Game/Blueprints/NPC/NPC.MeleeAttack` (`self.NPC`)))

(event `self.AIPerception.OnTargetPerceptionUpdated`
  (params (Actor :type "Actor Object Reference") (Stimulus :type "AIStimulus Structure"))
  ;[1 1 1] Searching for target
  (`BlackboardComponent.SetValueAsBool` (`AIBlueprintHelperLibrary.GetBlackboard` null) "CanSeeTarget" (`.bSuccessfullySensed` (break `AIStimulus` Stimulus))))

(fn `UserConstructionScript`)