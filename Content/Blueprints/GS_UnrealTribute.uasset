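; GS_UnrealTribute provides a shared area-of-effect query, SpawnAOE, that reports affected actors through a caller-supplied delegate, with optional debug drawing.
; It sphere-overlaps pawns, excluding the instigator, and binds the delegate only for the call's duration.
; Optional line-of-sight checks trace to each actor's bounds center and eight GetBoxCorners points, counting a hit on the first unblocked trace.
; GetBoxCorners returns top and bottom edge midpoints, using X extent for negative Y.
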(fn `GetBoxCorners`
  (params (Origin :type "Vector Structure") (BoxExtent :type "Vector Structure"))
  (returns (Corners :type "Array of Vector Structure"))
  (bind (_boxextent_x _boxextent_y _boxextent_z) (`KismetMathLibrary.BreakVector` (`local.BoxExtent`)))
  (bind (_boxextent_x_2 _boxextent_y_2 _boxextent_z_2) (`KismetMathLibrary.BreakVector` (`local.BoxExtent`)))
  (bind (_boxextent_x_3 _boxextent_y_3 _boxextent_z_3) (`KismetMathLibrary.BreakVector` (`local.BoxExtent`)))
  (bind (_boxextent_x_4 _boxextent_y_4 _boxextent_z_4) (`KismetMathLibrary.BreakVector` (`local.BoxExtent`)))
  (bind (_boxextent_x_5 _boxextent_y_5 _boxextent_z_5) (`KismetMathLibrary.BreakVector` (`local.BoxExtent`)))
  (bind (_boxextent_x_6 _boxextent_y_6 _boxextent_z_6) (`KismetMathLibrary.BreakVector` (`local.BoxExtent`)))
  (bind (_boxextent_x_7 _boxextent_y_7 _boxextent_z_7) (`KismetMathLibrary.BreakVector` (`local.BoxExtent`)))
  (bind (_boxextent_x_8 _boxextent_y_8 _boxextent_z_8) (`KismetMathLibrary.BreakVector` (`local.BoxExtent`)))
  (return (`|MakeArray` (`local.Origin`) (+ (`local.Origin`) (`KismetMathLibrary.MakeVector` _boxextent_x 0.0 _boxextent_z)) (+ (`local.Origin`) (`KismetMathLibrary.MakeVector` (* _boxextent_x_2 -1.0) 0.0 _boxextent_z_2)) (+ (`local.Origin`) (`KismetMathLibrary.MakeVector` 0.0 _boxextent_y_3 _boxextent_z_3)) (+ (`local.Origin`) (`KismetMathLibrary.MakeVector` 0.0 (* _boxextent_x_4 -1.0) _boxextent_z_4)) (+ (`local.Origin`) (`KismetMathLibrary.MakeVector` _boxextent_x_7 0.0 (* _boxextent_z_7 -1.0))) (+ (`local.Origin`) (`KismetMathLibrary.MakeVector` (* _boxextent_x_8 -1.0) 0.0 (* _boxextent_z_8 -1.0))) (+ (`local.Origin`) (`KismetMathLibrary.MakeVector` 0.0 _boxextent_y_6 (* _boxextent_z_6 -1.0))) (+ (`local.Origin`) (`KismetMathLibrary.MakeVector` 0.0 (* _boxextent_x_5 -1.0) (* _boxextent_z_5 -1.0))))))

(fn `SpawnAOE`
  (params (Location :type "Vector Structure") (Radius :type "Float (double-precision)") (`Require LOS` :type Boolean) (`AOE Instigator` :type "Actor Object Reference") (`Hit Delegate` :type "Delegate (by ref)") (DrawDebugDuration :type "Float (double-precision)") (DebugColor :type "LinearColor Structure"))
  (locals (CurrentActor :type "Actor Object Reference"))
  (bind (_origin _boxextent) (`self.GetActorBounds` (`local.CurrentActor`) true true))
  (add `self.AOE HIT Delegate` `Hit Delegate`)
  (`|ExecutionSequence`
    (:`then_0`
      (if (> (`local.DrawDebugDuration`) 0.0)
        (`KismetSystemLibrary.DrawDebugSphere` (`local.Location`) (`local.Radius`) 16 (`local.DebugColor`) (`local.DrawDebugDuration`) 2.0))
      (bind _outactors (`KismetSystemLibrary.SphereOverlapActors` (`local.Location`) (`local.Radius`) (`|MakeArray` "ObjectTypeQuery3" :!type "EObjectTypeQuery Enum") "/Script/Engine.Actor" (`|MakeArray` (`local.AOE Instigator`))))
      (for _array_element _outactors
        (bind _output_get (set `local.CurrentActor` _array_element))
        (if (`KismetSystemLibrary.DoesImplementInterface` _output_get)
          _
          (else
            _))
        (if (`local.Require LOS`)
          (bind _corners (`self.GetBoxCorners` _origin _boxextent))
          (for _array_element_2 _corners
            (bind (_outhit _returnvalue) (`KismetSystemLibrary.LineTraceSingle` (`local.Location`) _array_element_2 "TraceTypeQuery1" false (`|MakeArray` (`local.AOE Instigator`)) (select `bool` (> (`local.DrawDebugDuration`) 0.0) :`true` "ForDuration" :!type "EDrawDebugTrace Enum") true (struct :`R` 1.0 :`A` 1.0) (struct :`G` 1.0 :`A` 1.0) (`local.DrawDebugDuration`)))
            (if (not _returnvalue)
              (`self.AOE HIT Delegate` (`local.CurrentActor`))
              (break)))
          (else
            (`self.AOE HIT Delegate` (`local.CurrentActor`))))))
    (:`then_1`
      (remove `self.AOE HIT Delegate` (`local.Hit Delegate`)))))

(fn `UserConstructionScript`)